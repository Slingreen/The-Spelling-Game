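; BP_CustomPlayer is the overworld player actor, handling movement and the transition into combat.
; Right and up axis inputs feed MoveRight and MoveUp helpers, whose results set the actor's location directly without sweep.
; Any actor overlap calls EnterCombat, teleports the player to the NewTpLoc location, and swaps the first GameWold_HUD widget found for a new CombatUI_HUD, with no filter on the other actor.
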(event EventBeginPlay)

(event EventTick
  (params (DeltaSeconds :type Float%20%28single-precision%29)))

(event Collision|EventActorBeginOverlap
  (params (OtherActor :type Actor%20Object%20Reference))
  (Class|CustomPlayer|EnterCombat OtherActor)
  (bind _returnvalue (Class|CustomPlayer|NewTpLoc))
  (Transformation|SetActorLocation _returnvalue false true)
  (bind _foundwidgets (Widget|GetAllWidgetsOfClass "/Game/UV_v1/GameWold_HUD.GameWold_HUD_C" true))
  (bind _output_get (Variables|Default|SetOverworldUI _foundwidgets))
  (Widget|RemovefromParent (Utilities|Array|Get(acopy) _output_get))
  (bind _returnvalue_2 (UserInterface|CreateWidget "/Game/UV_v1/CombatUI_HUD.CombatUI_HUD_C"))
  (UserInterface|Viewport|AddtoViewport _returnvalue_2 0))

(event Input|AxisEvents|InputAxisRightMovement
  (params (AxisValue :type Float%20%28single-precision%29))
  ;[1 1 1] Movement
  (bind _returnvalue (Class|CustomPlayer|MoveRight AxisValue (Transformation|GetActorLocation) 35))
  (Transformation|SetActorLocation _returnvalue false false))

(event Input|AxisEvents|InputAxisUpMovement
  (params (AxisValue :type Float%20%28single-precision%29))
  ;[1 1 1] Movement
  (bind _returnvalue (Class|CustomPlayer|MoveUp AxisValue (Transformation|GetActorLocation) 35))
  (Transformation|SetActorLocation _returnvalue false false))

(fn ConstructionScript)