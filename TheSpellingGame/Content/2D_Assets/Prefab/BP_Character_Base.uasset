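; BP_Character_Base is a base Blueprint for a player-controlled character among the 2D assets, moved directly by axis input.
; On BeginPlay it enables input from player controller 0.
; The RightMovement and UpMovement axes pass the current location and a fixed adjustment to Move's MoveRight and MoveUp functions.
; Each result is applied with SetActorLocation without sweep, so movement does not stop at collisions.
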(event EventBeginPlay
  (Input|EnableInput (Game|GetPlayerController 0)))

(event Collision|EventActorBeginOverlap
  (params (OtherActor :type Actor%20Object%20Reference)))

(event Input|AxisEvents|InputAxisRightMovement
  (params (AxisValue :type Float%20%28single-precision%29))
  (bind _returnvalue (Class|CustomPlayerActions|MoveRight (Variables|Default|GetMove) AxisValue (Transformation|GetActorLocation) 35))
  (Transformation|SetActorLocation _returnvalue false false))

(event Input|AxisEvents|InputAxisUpMovement
  (params (AxisValue :type Float%20%28single-precision%29))
  (bind _returnvalue (Class|CustomPlayerActions|MoveUp (Variables|Default|GetMove) AxisValue (Transformation|GetActorLocation) 35))
  (Transformation|SetActorLocation _returnvalue false false))

(fn ConstructionScript)